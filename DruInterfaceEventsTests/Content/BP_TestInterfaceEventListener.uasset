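; A test listener Blueprint that subscribes to a value-changed event exposed through an interface on a given broadcaster.
; Separate bind events attach either a regular or a const handler, and both store the received value in LastEventValue.
; Companion events remove a single binding or clear all bindings on the broadcaster through interface calls.
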(event `self.BindToEvent`
  (params (Broadcaster :type "TestBroadcaster Interface (by ref)"))
  (`|InterfaceEventAdd` Broadcaster (delegate `OnValueChanged`)))

(event `OnValueChanged`
  (params (NewValue :type Integer))
  (set `self.LastEventValue` NewValue))

(event `self.BindToEventConst`
  (params (Broadcaster :type "TestBroadcaster Interface (by ref)"))
  (`|InterfaceEventAdd` Broadcaster (delegate `OnValueChangedConst`)))

(event `OnValueChangedConst`
  (params (NewValue :type Integer))
  (set `self.LastEventValue` NewValue))

(event `self.UnbindFromEvent`
  (params (Broadcaster :type "TestBroadcaster Interface (by ref)"))
  (`|InterfaceEventRemove` Broadcaster (`|CreateDelegate` :!event `OnValueChanged`)))

(event `self.UnbindAllFromEvent`
  (params (Broadcaster :type "TestBroadcaster Interface (by ref)"))
  (`|InterfaceEventRemoveAll` Broadcaster))